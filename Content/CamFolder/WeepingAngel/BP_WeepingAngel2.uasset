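; BP_WeepingAngel2 is a Weeping Angel character that, as wired, only loops a head-shaking animation on BeginPlay.
; Tick, overlap and KillAngel are empty.
; Disconnected leftover nodes hold the stalker logic: chase the player unless watched, using a view dot product and a line trace for blocking walls.
; Other unreachable nodes cover movement audio, shutdown, and a death sound with a game-over level load.
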(event `self.ReceiveBeginPlay`
  (`SkeletalMeshComponent.PlayAnimation` (`self.Mesh`) "/Game/Alex/Assets/Animation/Shaking_Head_No.Shaking_Head_No" true))

(event `self.ReceiveTick`
  (params (DeltaSeconds :type "Float (single-precision)")))

(event `KillAngel`)

(fn `UserConstructionScript`)