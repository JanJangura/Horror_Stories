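; BP_WeepingAngel is a Weeping Angel enemy that chases the player only while unseen and opens the game-over level when its trigger overlaps them.
; Each Tick, a facing dot product and camera visibility trace, ignoring "Collision"-tagged actors, choose between AI MoveTo and stopping.
; KillAngel deactivates movement and the trigger, then plays a looping running animation.
; Sound logic is left unconnected.
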(event `self.ReceiveTick`
  (params (DeltaSeconds :type "Float (single-precision)"))
  (bind _returnvalue (`GameplayStatics.GetPlayerCharacter` 0))
  (if (> (`KismetMathLibrary.Dot_VectorVector` (`KismetMathLibrary.Normal` (- (`self.K2_GetActorLocation`) (`self.K2_GetActorLocation` _returnvalue))) (`self.GetActorForwardVector` _returnvalue)) 0.7)
    (bind _outactors (`GameplayStatics.GetAllActorsWithTag` "Collision"))
    ;[1 1 1] if the player is looking at the NPC the the NPC can move if a wall is in the way
    (bind (_outhit _returnvalue_2) (`KismetSystemLibrary.LineTraceSingle` (`PlayerCameraManager.GetCameraLocation` (`GameplayStatics.GetPlayerCameraManager` 0)) (`self.K2_GetActorLocation`) "TraceTypeQuery1" false _outactors))
    (if _returnvalue_2
      (`|AIMoveTo` self (0.0 0.0 0.0) (`GameplayStatics.GetPlayerCharacter` 0) :!label _label)
      (else
        (`MovementComponent.StopMovementImmediately` (`self.CharacterMovement`))))
    (else
      (goto _label))))

(event `Play Sound`)

(event `self.Player hit trigger.OnComponentBeginOverlap`
  (params (OverlappedComponent :type "PrimitiveComponent Object Reference") (OtherActor :type "Actor Object Reference") (OtherComp :type "PrimitiveComponent Object Reference") (OtherBodyIndex :type Integer) (bFromSweep :type Boolean) (SweepResult :type "HitResult Structure (by ref)"))
  (cast `/Game/FirstPerson/Blueprints/BP_FirstPersonCharacter` OtherActor)
  (`GameplayStatics.OpenLevelBySoftObjectPtr` "/Game/CamFolder/WeepingAngel/WeepingAngelGameOverLevel.WeepingAngelGameOverLevel"))

(event `KillAngel`
  (`ActorComponent.Deactivate` (`self.CharacterMovement`))
  (`ActorComponent.Deactivate` (`self.Player hit trigger`))
  (`MovementComponent.StopMovementImmediately` (`self.CharacterMovement`))
  (`NavMovementComponent.StopActiveMovement` (`self.CharacterMovement`))
  (`SkeletalMeshComponent.PlayAnimation` (`self.Mesh`) "/Game/CamFolder/WeepingAngel/animations/Running__1_.Running__1_" true))

(fn `UserConstructionScript`)