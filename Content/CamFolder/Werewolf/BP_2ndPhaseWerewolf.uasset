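; Second-phase werewolf enemy that heads straight for the player on spawn and opens the Weeping Angel game-over level on touching them.
; AI MoveTo drives movement; StopChase drops it into a slower, looping patrol toward the first patrol location.
; Shots drain health; death flags the elimination on the game mode, checks the win condition and disables the werewolf atmosphere.
; StartChase only sets a detection flag, as pawn-sensing detection logic is disconnected.
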(event `self.ReceiveBeginPlay`
  (`PrimitiveComponent.SetMaterial` (`self.Mesh`) 0 "/Game/CamFolder/WeepingAngel/RedForBox.RedForBox")
  (set `CharacterMovementComponent.MaxWalkSpeed` 400.0 (`self.CharacterMovement`))
  (`|AIMoveTo` self (0.0 0.0 0.0) (`GameplayStatics.GetPlayerCharacter` 0)))

(event `self.PawnSensing.OnSeePawn`
  (params (Pawn :type "Pawn Object Reference")))

(event `self.startChase`
  (set `self.isDectected` true))

(event `self.stopChase`
  (set `self.isDectected` false)
  (`|AIMoveTo` self (0.0 0.0 0.0) self
    (:`then`
      (`self.Patrol`))))

(event `Patrol`
  ;[1 1 1] Patrol
  (set `CharacterMovementComponent.MaxWalkSpeed` 230.0 (`self.CharacterMovement`))
  (`|AIMoveTo` self (`|GetArrayItem` (`self.Patrol Location`)) null
    (:`OnSuccess`
      (if (not (`self.isDectected`))
        (`KismetSystemLibrary.Delay` (`KismetMathLibrary.RandomFloatInRange` 1.0 2.0))
        (`self.Patrol`)))))

(event `self.PlayerHitTrigger.OnComponentBeginOverlap`
  (params (OverlappedComponent :type "PrimitiveComponent Object Reference") (OtherActor :type "Actor Object Reference") (OtherComp :type "PrimitiveComponent Object Reference") (OtherBodyIndex :type Integer) (bFromSweep :type Boolean) (SweepResult :type "HitResult Structure (by ref)"))
  (bind _asbp_first_person_character (cast `/Game/FirstPerson/Blueprints/BP_FirstPersonCharacter` OtherActor))
  (if (`KismetSystemLibrary.IsValid` _asbp_first_person_character)
    (`GameplayStatics.OpenLevelBySoftObjectPtr` "/Game/CamFolder/WeepingAngel/WeepingAngelGameOverLevel.WeepingAngelGameOverLevel")))

(event `self.Werewolf Shot`
  (bind _game_mode (`self.Game Mode`))
  (bind _result (`/Engine/EditorBlueprintResources/StandardMacros.DecrementInt` (`self.Health`))
    (:`  `
      (`KismetSystemLibrary.PrintString` "HIT!")
      (if (<= _result 0)
        (set `/Game/FirstPerson/Blueprints/BP_FirstPersonGameMode.Werewolf Eliminated` true _game_mode)
        (`/Game/FirstPerson/Blueprints/BP_FirstPersonGameMode.WinCondition` _game_mode)
        (`self.K2_DestroyActor`)
        (bind _outactors (`GameplayStatics.GetAllActorsOfClass` "/Game/ZoeFolder/BPAtmosphereChanges.BPAtmosphereChanges_C"))
        (`/Game/ZoeFolder/BPAtmosphereChanges.WerewolfAtmosDisabled` (`|GetArrayItem` _outactors))))))

(event `GameModeRef`
  (params (GameMode :type "/Game/FirstPerson/Blueprints/BP_FirstPersonGameMode Object Reference"))
  (`/Engine/EditorBlueprintResources/StandardMacros.IsValid` GameMode
    (:`Is Valid`
      (set `self.Game Mode` GameMode))))

(fn `UserConstructionScript`)