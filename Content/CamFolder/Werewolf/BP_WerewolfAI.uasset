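; Werewolf enemy that patrols random points, hunts the player, and triggers a jumpscare and game-over level on contact.
; PawnSensing starts the player's detection message and freezes the wolf; a retriggerable delay clears it when sight is lost.
; External StartChase and StopChase events switch between pursuit and patrol.
; Shots drain health until a second phase disables sensing, turns it red, raises its speed and sends it after the shooter.
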(event `2ndPhase`
  (bind _mesh (`self.Mesh`))
  (set `self.SecondPhase` true)
  (`ActorComponent.Deactivate` (`self.PawnSensing`))
  (`PrimitiveComponent.SetMaterial` _mesh 2 "/Game/CamFolder/WeepingAngel/RedForBox.RedForBox")
  (`PrimitiveComponent.SetMaterial` _mesh 0 "/Game/CamFolder/WeepingAngel/RedForBox.RedForBox")
  (set `CharacterMovementComponent.MaxWalkSpeed` 500.0 (`self.CharacterMovement`))
  (`|AIMoveTo` self (0.0 0.0 0.0) (`self.Character`)))

(event `self.ReceiveBeginPlay`
  (`self.Patrol`))

(event `self.PawnSensing.OnSeePawn`
  (params (Pawn :type "Pawn Object Reference"))
  (if (not (`self.SecondPhase`))
    (`|ExecutionSequence`
      (:`then_0`
        (`|ExecutionSequence`
          (:`then_0`
            (`/Engine/EditorBlueprintResources/StandardMacros.DoOnce` false :!label _label
              (:`Completed`
                (set `self.isSensing` true)
                (`self.FlopWerewolfMovement`)
                (message `/Game/CamFolder/Werewolf/BPI_WerewolfDection.startDection` Pawn self))))
          (:`then_1`
            (if (`self.isDectected`)
              (`|AIMoveTo` self (0.0 0.0 0.0) Pawn)))))
      (:`then_1`
        (`KismetSystemLibrary.RetriggerableDelay` 0.2)
        (message `/Game/CamFolder/Werewolf/BPI_WerewolfDection.stopDection` Pawn)
        (`self.FlopWerewolfMovement`)
        (goto _label :!via `Reset`)))))

(event `FlopWerewolfMovement`
  (bind _charactermovement (`self.CharacterMovement`))
  (if (and (`self.isSensing`) (not (`self.isDectected`)))
    (`CharacterMovementComponent.DisableMovement` _charactermovement)
    (else
      (`CharacterMovementComponent.SetMovementMode` _charactermovement "MOVE_Walking" 0))))

(event `/Game/CamFolder/Werewolf/BPI_WerewolfDection.startChase`
  (set `self.isSensing` false)
  (set `self.isDectected` true)
  (`self.FlopWerewolfMovement`))

(event `/Game/CamFolder/Werewolf/BPI_WerewolfDection.stopChase`
  (set `self.isSensing` false)
  (set `self.isDectected` false)
  (`self.FlopWerewolfMovement`)
  (`|AIMoveTo` self (0.0 0.0 0.0) self
    (:`then`
      (`KismetSystemLibrary.Delay` 0.2)
      (`self.Patrol`))))

(event `Patrol`
  (bind _patrol_location (`self.Patrol Location`))
  ;[1 1 1] Patrol
  (if (not (`self.SecondPhase`))
    (`|AIMoveTo` self (`|GetArrayItem` _patrol_location (`KismetMathLibrary.RandomIntegerInRange` 0 (`KismetMathLibrary.FTrunc` (`KismetMathLibrary.Conv_IntToDouble` (`KismetArrayLibrary.Array_Length` _patrol_location))))) null
      (:`OnSuccess`
        (if (not (`self.isDectected`))
          (`KismetSystemLibrary.Delay` 5.0)
          (`self.Patrol`))))
    (else
      (`self.RunToForest`))))

(event `self.PlayerHitTrigger.OnComponentBeginOverlap`
  (params (OverlappedComponent :type "PrimitiveComponent Object Reference") (OtherActor :type "Actor Object Reference") (OtherComp :type "PrimitiveComponent Object Reference") (OtherBodyIndex :type Integer) (bFromSweep :type Boolean) (SweepResult :type "HitResult Structure (by ref)"))
  (bind _asbp_first_person_character (cast `/Game/FirstPerson/Blueprints/BP_FirstPersonCharacter` OtherActor))
  (if (`KismetSystemLibrary.IsValid` _asbp_first_person_character)
    (bind _asbp_first_person_character_2 (cast `/Game/FirstPerson/Blueprints/BP_FirstPersonCharacter` OtherActor))
    (`GameplayStatics.PlaySound2D` "/Game/ZoeFolder/wolf-howling-type-04-293317.wolf-howling-type-04-293317" 1.0 1.0 0.0 null null)
    (`self.DisableInput` _asbp_first_person_character_2 null)
    (`SceneComponent.ToggleVisibility` (`self.Mesh`) false)
    (`SceneComponent.ToggleVisibility` (`/Game/FirstPerson/Blueprints/BP_FirstPersonCharacter.JumpScareREF` _asbp_first_person_character_2) false)
    (`SkeletalMeshComponent.PlayAnimation` (`self.Mesh`) "/Game/Werewolf/Demo/Animations/ThirdPerson_Jump.ThirdPerson_Jump" false)
    (`KismetSystemLibrary.Delay` 5.0)
    (`GameplayStatics.OpenLevelBySoftObjectPtr` "/Game/CamFolder/WeepingAngel/WeepingAngelGameOverLevel.WeepingAngelGameOverLevel")))

(event `/Game/Alex/Blueprints/BPI_Werewolf_A.Werewolf Shot`
  (params (Player :type "/Game/FirstPerson/Blueprints/BP_FirstPersonCharacter Object Reference"))
  (bind _output_get (set `self.Character` Player))
  (`/Engine/EditorBlueprintResources/StandardMacros.IsValid` _output_get
    (:`Is Valid`
      (`KismetSystemLibrary.PrintString` "Valid"))
    (:`Is Not Valid`
      (`KismetSystemLibrary.PrintString` "Not Valid")))
  (bind _result (`/Engine/EditorBlueprintResources/StandardMacros.DecrementInt` (`self.Health`))
    (:`  `
      (`KismetSystemLibrary.PrintString` "HIT!")
      (if (<= _result 0)
        (`self.2ndPhase`)))))

(event `GameModeRef`
  (params (GameMode :type "/Game/FirstPerson/Blueprints/BP_FirstPersonGameMode Object Reference"))
  (`/Engine/EditorBlueprintResources/StandardMacros.IsValid` GameMode
    (:`Is Valid`
      (set `self.Game Mode` GameMode))))

(event `RunToForest`
  (`/Game/CamFolder/Werewolf/BPI_WerewolfDection.stopDection`)
  (`|AIMoveTo` self (`self.Location`) null))

(fn `UserConstructionScript`)