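; BP_GhostSlow is a ghost enemy that moves toward the player and triggers an object possession when the camera interacts with it.
; BeginPlay issues a single AIMoveTo targeting the player character.
; CameraInteract, gated by DoOnce, calls PossissionState on a random BP_PossessableObj, using an inclusive range that can overrun the array by one.
; Chase and PawnSensing events are empty, with leftover chase logic disconnected.
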(event `self.ReceiveBeginPlay`
  (`|AIMoveTo` self (0.0 0.0 0.0) (`GameplayStatics.GetPlayerCharacter` 0)))

(event `self.ReceiveTick`
  (params (DeltaSeconds :type "Float (single-precision)")))

(event `CameraInteract`
  (`/Engine/EditorBlueprintResources/StandardMacros.DoOnce` false
    (:`Completed`
      (bind _outactors (`GameplayStatics.GetAllActorsOfClass` "/Game/CamFolder/Ghost/BP_PossessableObj.BP_PossessableObj_C"))
      (`/Game/CamFolder/Ghost/BP_PossessableObj.PossissionState` (`|GetArrayItem` _outactors (`KismetMathLibrary.RandomIntegerInRange` 0 (`KismetArrayLibrary.Array_Length` _outactors)))))))

(event `Chase`)

(event `self.PawnSensing.OnSeePawn`
  (params (Pawn :type "Pawn Object Reference")))

(fn `UserConstructionScript`)