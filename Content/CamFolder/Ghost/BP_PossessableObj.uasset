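; BP_PossessableObj is an object that a ghost can possess, giving the player a timed window to eliminate it.
; PossissionState shows a possession effect, plays clock ticking and starts a 30-second timer to Captured, which spawns BP_Ghost1 at a random BP_LocationRef.
; PossessedItem, while possessed, notifies the game mode of the elimination and sets GhostIsSpawned, blocking that respawn.
; Overlap and Interact events are empty, and several older logic chains are disconnected.
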(event `Timer`)

(event `self.ReceiveBeginPlay`
  (`ActorComponent.Deactivate` (`self.DefaultSceneRoot`))
  (`KismetSystemLibrary.PrintString` "Deactivated")
  (`SceneComponent.SetVisibility` (`self.possess_PE`) false false))

(event `Key|J`
  (params (Key :type "Key Structure")))

(event `NotCaptured`)

(event `Captured`
  (if (not (`self.ghostIsSpawned`))
    (set `self.ghostIsSpawned` true)
    (set `self.isPossessed` false)
    (`AudioComponent.Stop` (`self.Clock_Ticking`))
    (bind _outactors (`GameplayStatics.GetAllActorsOfClass` "/Game/Alex/Blueprints/BP_LocationRef.BP_LocationRef_C"))
    (`|SpawnActorFromClass` "/Game/CamFolder/Ghost/BP_Ghost1.BP_Ghost1_C" (`KismetMathLibrary.Conv_VectorToTransform` (`self.K2_GetActorLocation` (`|GetArrayItem` _outactors (`KismetMathLibrary.RandomIntegerInRange` 0 (- (`KismetArrayLibrary.Array_Length` _outactors) 1))))) "Undefined" "MultiplyWithRoot" null null)
    (`SceneComponent.SetVisibility` (`self.possess_PE`) false false)))

(event `PossissionState`
  (set `self.ghostIsSpawned` false)
  (set `self.isPossessed` true)
  (`KismetSystemLibrary.PrintString` (`KismetSystemLibrary.GetDisplayName` self))
  (`ActorComponent.Activate` (`self.DefaultSceneRoot`) false)
  (`SceneComponent.SetVisibility` (`self.possess_PE`) true false)
  (`AudioComponent.Play` (`self.Clock_Ticking`) 0.0)
  (`KismetSystemLibrary.K2_SetTimerDelegate` (delegate `Captured`) 30.0))

(event `Chase`
  (params (`Ghost Ref` :type "/Game/CamFolder/Ghost/BP_Ghost1 Object Reference"))
  (bind _returnvalue (`GameplayStatics.GetActorOfClass` (`GameplayStatics.GetObjectClass` `Ghost Ref`)))
  (`|AIMoveTo` _returnvalue (0.0 0.0 0.0) _returnvalue))

(event `self.ExitBox.OnComponentEndOverlap`
  (params (OverlappedComponent :type "PrimitiveComponent Object Reference") (OtherActor :type "Actor Object Reference") (OtherComp :type "PrimitiveComponent Object Reference") (OtherBodyIndex :type Integer)))

(event `self.EnterBox.OnComponentBeginOverlap`
  (params (OverlappedComponent :type "PrimitiveComponent Object Reference") (OtherActor :type "Actor Object Reference") (OtherComp :type "PrimitiveComponent Object Reference") (OtherBodyIndex :type Integer) (bFromSweep :type Boolean) (SweepResult :type "HitResult Structure (by ref)")))

(event `/Game/CamFolder/WeepingAngel/BPI_Interact.PossessedItem`
  (params (FirstPersonCharacter :type "/Game/FirstPerson/Blueprints/BP_FirstPersonCharacter Object Reference"))
  (if (`self.isPossessed`)
    (set `self.ghostIsSpawned` true)
    (`/Game/FirstPerson/Blueprints/BP_FirstPersonGameMode.GhostisEliminated` (`/Game/FirstPerson/Blueprints/BP_FirstPersonCharacter.GameMode` FirstPersonCharacter) null)
    (`SceneComponent.ToggleVisibility` (`self.possess_PE`) false)))

(event `/Game/CamFolder/WeepingAngel/BPI_Interact.Interact`)

(fn `UserConstructionScript`)