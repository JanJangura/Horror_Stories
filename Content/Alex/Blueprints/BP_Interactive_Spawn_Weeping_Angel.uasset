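; One-shot interactable that starts the Weeping Angel monster encounter.
; On BeginPlay it registers its Cube as the GameMode's Weeping Angel spawn mesh.
; First interaction turns off the overlay, sets the player's monster state and enables atmosphere saturation, then after a delay spawns BP_WeepingAngel at a hardcoded location with a scrape sound and registers it with the GameMode.
; An InteractedAlready flag blocks repeats and switches the reported interactable type.
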(event `self.ReceiveBeginPlay`
  (bind _gamemode (`self.GameMode`))
  (`parent.ReceiveBeginPlay`)
  (bind _output_get (set `/Game/FirstPerson/Blueprints/BP_FirstPersonGameMode.SpawnMeshWeepingAngel` (`self.Cube`) _gamemode))
  (`KismetArrayLibrary.Array_AddUnique` (`/Game/FirstPerson/Blueprints/BP_FirstPersonGameMode.SpawnMeshes` _gamemode) _output_get))

(event `/Game/Alex/Blueprints/BPI_ObjectInteract.ObjectInteract`
  (params (PlayerCharacter :type "/Game/FirstPerson/Blueprints/BP_FirstPersonCharacter Object Reference"))
  (bind _gamemode (`/Game/FirstPerson/Blueprints/BP_FirstPersonCharacter.GameMode` (`self.Player Character`)))
  (if (not (`self.InteractedAlready`))
    (set `self.InteractedAlready` true)
    (`self.TurnOffOverlay`)
    (`/Engine/EditorBlueprintResources/StandardMacros.IsValid` PlayerCharacter
      (:`Is Valid`
        (bind _output_get (set `self.Player Character` PlayerCharacter))
        (set `/Game/FirstPerson/Blueprints/BP_FirstPersonCharacter.CurrentMonsterState` (`self.WeepingAngel_State`) _output_get)
        (`self.InteractionTrigger` _output_get)
        (`self.EventObjectInUse` _output_get)
        (`/Engine/EditorBlueprintResources/StandardMacros.IsValid` _gamemode
          (:`Is Valid`
            (bind _outactors (`GameplayStatics.GetAllActorsOfClass` "/Game/ZoeFolder/BPAtmosphereChanges.BPAtmosphereChanges_C"))
            (`/Game/ZoeFolder/BPAtmosphereChanges.WASaturationEnabled` (`|GetArrayItem` _outactors))
            (`KismetSystemLibrary.Delay` 6.0)
            (bind _returnvalue (`|SpawnActorFromClass` "/Game/CamFolder/WeepingAngel/BP_WeepingAngel.BP_WeepingAngel_C" (`KismetMathLibrary.MakeTransform` (-949.678077 -373.475806 701.545827)) "Undefined" "MultiplyWithRoot" null null))
            (`/Game/FirstPerson/Blueprints/BP_FirstPersonGameMode.Add Weeping Angel` _gamemode _returnvalue)
            (`GameplayStatics.SpawnSoundAtLocation` "/Game/CamFolder/Sounds/Concrete_scrape_loop.Concrete_scrape_loop" (-949.0 -373.0 700.0) (struct) 1.0 1.0 0.0 null null)))))))

(fn `GetInteractableType`
  (returns (`Actor Enum` :type "/Game/Alex/Blueprints/Enum_Interactive_Object_Types Enum"))
  (locals (Off :type Boolean))
  (if (`self.Interacted Already`)
    (return "NewEnumerator3")
    (else
      (return "NewEnumerator0"))))

(fn `UserConstructionScript`
  (`parent.UserConstructionScript`))