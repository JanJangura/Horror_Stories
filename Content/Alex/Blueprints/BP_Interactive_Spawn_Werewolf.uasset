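; Interactive werewolf spawn point that registers its Cube mesh with the game mode on BeginPlay.
; Its one-time interaction spawns a second-phase werewolf, sets the player's monster state and starts the game mode's werewolf sequence.
; A separate SpawnWerewolfAI event plays a howl, spawns and registers the AI werewolf, and destroys the shed doors.
; The reported interactable type changes once the object has been used.
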(event `self.ReceiveBeginPlay`
  (bind _gamemode (`self.GameMode`))
  (`parent.ReceiveBeginPlay`)
  (bind _output_get (set `/Game/FirstPerson/Blueprints/BP_FirstPersonGameMode.SpawnMeshWerewolf` (`self.Cube`) _gamemode))
  (`KismetArrayLibrary.Array_AddUnique` (`/Game/FirstPerson/Blueprints/BP_FirstPersonGameMode.SpawnMeshes` _gamemode) _output_get)
  (`/Game/FirstPerson/Blueprints/BP_FirstPersonGameMode.AddSpawningMesh` _gamemode (`self.Cube`)))

(event `self.ObjectInteract`
  (params (PlayerCharacter :type "/Game/FirstPerson/Blueprints/BP_FirstPersonCharacter Object Reference"))
  (bind _gamemode (`self.GameMode`))
  (if (not (`self.InteractedAlready`))
    (set `self.InteractedAlready` true)
    (`self.TurnOffOverlay`)
    (`|SpawnActorFromClass` :`Class` "/Game/CamFolder/Werewolf/BP_2ndPhaseWerewolf.BP_2ndPhaseWerewolf_C" :`SpawnTransform` (`self.TRANSFORM`) :`CollisionHandlingOverride` "Undefined" :`TransformScaleMethod` "MultiplyWithRoot" :`Instigator` null)
    (`/Engine/EditorBlueprintResources/StandardMacros.IsValid` PlayerCharacter
      (:`Is Valid`
        (bind _output_get (set `self.Player Character` PlayerCharacter))
        (set `/Game/FirstPerson/Blueprints/BP_FirstPersonCharacter.CurrentMonsterState` (`self.Werewolf_State`) _output_get)
        (`self.InteractionTrigger` _output_get)
        (`self.EventObjectInUse` _output_get)
        (`/Engine/EditorBlueprintResources/StandardMacros.IsValid` _gamemode
          (:`Is Valid`
            (`/Game/FirstPerson/Blueprints/BP_FirstPersonGameMode.Player_Interactive_Werewolf_Sequence` _gamemode self)))))))

(event `Spawn Werewolf AI`
  (bind _location (`self.Location`))
  (`GameplayStatics.SpawnSoundAtLocation` "/Game/ZoeFolder/wolf-howling-type-04-293317.wolf-howling-type-04-293317" _location (struct) 1.0 1.0 0.0 null null)
  (bind _returnvalue (`|SpawnActorFromClass` :`Class` "/Game/CamFolder/Werewolf/BP_WerewolfAI.BP_WerewolfAI_C" :`SpawnTransform` (`KismetMathLibrary.MakeTransform` _location (struct :`Yaw` 15.0)) :`CollisionHandlingOverride` "Undefined" :`TransformScaleMethod` "MultiplyWithRoot" :`Instigator` null))
  (`/Game/FirstPerson/Blueprints/BP_FirstPersonGameMode.Add Werewolf` (`self.GameMode`) _returnvalue)
  (bind _outactors (`GameplayStatics.GetAllActorsOfClass` "/Game/ZoeFolder/BPshedDoor.BPshedDoor_C"))
  (`self.K2_DestroyActor` _outactors))

(fn `GetInteractableType`
  (returns (`Actor Enum` :type "/Game/Alex/Blueprints/Enum_Interactive_Object_Types Enum"))
  (if (`self.Interacted Already`)
    (return "NewEnumerator3")
    (else
      (return "NewEnumerator1"))))

(fn `UserConstructionScript`
  (`parent.UserConstructionScript`))