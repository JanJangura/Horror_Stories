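; BP_Gun_A is an interactable gun pickup that the player can use to shoot a werewolf.
; Interacting in the required monster state stores the player, passes the gun to them and disables its collision.
; Fireweapon spawns a Niagara muzzle flash and runs a debug-drawn, short-range camera line trace.
; A hit on a BPI_Werewolf_A implementer sends the shot message, then the gun destroys itself.
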(event `/Game/Alex/Blueprints/BPI_ObjectInteract.ObjectInteract`
  (params (PlayerCharacter :type "/Game/FirstPerson/Blueprints/BP_FirstPersonCharacter Object Reference"))
  (if (`|EnumEquality` (`/Game/FirstPerson/Blueprints/BP_FirstPersonCharacter.CurrentMonsterState` PlayerCharacter) "NewEnumerator2")
    (bind _output_get (set `self.PlayerCharacter` PlayerCharacter))
    (`/Game/FirstPerson/Blueprints/BP_FirstPersonCharacter.GunRef` _output_get self)
    (`PrimitiveComponent.SetCollisionEnabled` (`self.Collision`) "NoCollision")))

(event `/Game/CamFolder/WeepingAngel/BPI_Interact.Interact`)

(fn `Fireweapon`
  (bind _playercharacter (`self.PlayerCharacter`))
  (bind _firstpersoncamera (`/Game/FirstPerson/Blueprints/BP_FirstPersonCharacter.FirstPersonCamera` _playercharacter))
  (bind _returnvalue (`SceneComponent.K2_GetComponentLocation` _firstpersoncamera))
  (`/Engine/EditorBlueprintResources/StandardMacros.IsValid` _playercharacter
    (:`Is Valid`
      (`NiagaraFunctionLibrary.SpawnSystemAtLocation` "/Game/MuzzleFlash/MuzzleFlash/Niagara/NS_MuzzleFlash.NS_MuzzleFlash" (`SceneComponent.K2_GetComponentLocation` (`self.GunEnd`)) (`KismetMathLibrary.MakeRotFromY` (`SceneComponent.GetForwardVector` (`Actor.RootComponent` (`self.PlayerCharacter`)))))
      (`KismetSystemLibrary.PrintString` "ParticleEffect?")
      (bind _outhit (`KismetSystemLibrary.LineTraceSingle` :`Start` _returnvalue :`End` (+ _returnvalue (* (`SceneComponent.GetForwardVector` _firstpersoncamera) 1000.0)) :`TraceChannel` "TraceTypeQuery1" :`DrawDebugType` "ForDuration"))
      (bind (_bblockinghit _binitialoverlap _time _distance _location _impactpoint _normal _impactnormal _physmat _hitactor) (`GameplayStatics.BreakHitResult` _outhit))
      (if (`KismetSystemLibrary.DoesImplementInterface` _hitactor "/Game/Alex/Blueprints/BPI_Werewolf_A.BPI_Werewolf_A_C")
        (message `/Game/Alex/Blueprints/BPI_Werewolf_A.Werewolf Shot` _hitactor)
        (`self.K2_DestroyActor`)))))

(fn `GetInteractableType`
  (returns (`Actor Enum` :type "/Game/Alex/Blueprints/Enum_Interactive_Object_Types Enum"))
  (return "NewEnumerator4"))

(fn `UserConstructionScript`)