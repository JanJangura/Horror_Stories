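; BP_Bullets_Alex is an interactable bullets pickup that shows a widget while something overlaps its sphere.
; The widget starts hidden and toggles on the sphere's begin and end overlap, with no filter on the overlapping actor.
; ObjectInteract sets HasBullets on the player character and destroys the pickup, but only when CurrentMonsterState matches one specific enum value.
; GetInteractableType reports a fixed type, and the plain Interact event is empty.
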(event `self.ReceiveBeginPlay`
  (`SceneComponent.SetVisibility` (`self.Widget`) false false))

(event `/Game/CamFolder/WeepingAngel/BPI_Interact.Interact`)

(event `/Game/Alex/Blueprints/BPI_ObjectInteract.ObjectInteract`
  (params (PlayerCharacter :type "/Game/FirstPerson/Blueprints/BP_FirstPersonCharacter Object Reference"))
  (if (`|EnumEquality` (`/Game/FirstPerson/Blueprints/BP_FirstPersonCharacter.CurrentMonsterState` PlayerCharacter) "NewEnumerator2")
    (set `/Game/FirstPerson/Blueprints/BP_FirstPersonCharacter.HasBullets` true PlayerCharacter)
    (`self.K2_DestroyActor`)))

(event `self.Sphere1.OnComponentBeginOverlap`
  (params (OverlappedComponent :type "PrimitiveComponent Object Reference") (OtherActor :type "Actor Object Reference") (OtherComp :type "PrimitiveComponent Object Reference") (OtherBodyIndex :type Integer) (bFromSweep :type Boolean) (SweepResult :type "HitResult Structure (by ref)"))
  (`SceneComponent.SetVisibility` (`self.Widget`) true false))

(event `self.Sphere1.OnComponentEndOverlap`
  (params (OverlappedComponent :type "PrimitiveComponent Object Reference") (OtherActor :type "Actor Object Reference") (OtherComp :type "PrimitiveComponent Object Reference") (OtherBodyIndex :type Integer))
  (`SceneComponent.SetVisibility` (`self.Widget`) false false))

(fn `GetInteractableType`
  (returns (`Actor Enum` :type "/Game/Alex/Blueprints/Enum_Interactive_Object_Types Enum"))
  (return "NewEnumerator0"))

(fn `UserConstructionScript`)