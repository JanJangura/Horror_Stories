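; BP_SpawnGhost is a one-time interactable that triggers the ghost phase of the game.
; On interaction it puts the player into the ghost monster state and runs the interaction events.
; If the player's game mode is valid, after a delay it plays a ghost sound at a fixed location and enables ghost atmosphere on BPAtmosphereChanges.
; Its interactable type changes once used; the actual ghost spawn node is disconnected.
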(event `self.ObjectInteract`
  (params (PlayerCharacter :type "/Game/FirstPerson/Blueprints/BP_FirstPersonCharacter Object Reference"))
  (if (not (`self.InteractedAlready`))
    (`/Engine/EditorBlueprintResources/StandardMacros.IsValid` PlayerCharacter
      (:`Is Valid`
        (bind _output_get (set `self.Player Character` PlayerCharacter))
        (set `/Game/FirstPerson/Blueprints/BP_FirstPersonCharacter.CurrentMonsterState` (`self.Ghost_State`) _output_get)
        (set `self.InteractedAlready` true)
        (`self.InteractionTrigger` _output_get)
        (`self.EventObjectInUse` _output_get)
        (`/Engine/EditorBlueprintResources/StandardMacros.IsValid` (`/Game/FirstPerson/Blueprints/BP_FirstPersonCharacter.GameMode` (`self.Player Character`))
          (:`Is Valid`
            (`KismetSystemLibrary.Delay` 6.0)
            (`GameplayStatics.SpawnSoundAtLocation` "/Game/Sound/ghost-6979.ghost-6979" (-949.0 -373.0 700.0) (struct) 1.0 1.0 0.0 null null)
            (bind _outactors (`GameplayStatics.GetAllActorsOfClass` "/Game/ZoeFolder/BPAtmosphereChanges.BPAtmosphereChanges_C"))
            (`/Game/ZoeFolder/BPAtmosphereChanges.GhostAtmosEnabled` (`|GetArrayItem` _outactors))))))))

(fn `GetInteractableType`
  (returns (`Actor Enum` :type "/Game/Alex/Blueprints/Enum_Interactive_Object_Types Enum"))
  (locals (Off :type Boolean))
  (if (`self.Interacted Already`)
    (return "NewEnumerator3")
    (else
      (return "NewEnumerator2"))))

(fn `UserConstructionScript`
  (`parent.UserConstructionScript`))