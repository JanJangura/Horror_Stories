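; BP_Interactive_Object is an interactable object that records whether the player has already interacted with it.
; Both interaction events set an InteractedAlready flag, and InteractionTrigger also stores the player character.
; EventObjectInUse sets ObjInUse on a valid player character.
; GetInteractableType is meant to classify monster spawning from that flag, but both branches currently return the same enum value.
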(event `/Game/Alex/Blueprints/BPI_ObjectInteract.ObjectInteract`
  (params (PlayerCharacter :type "/Game/FirstPerson/Blueprints/BP_FirstPersonCharacter Object Reference"))
  ;[1 0 0] Let's us know that the User has already interacted with this object
  (set `self.Interacted Already` true))

(event `InteractionTrigger`
  (params (PlayerCharacter :type "/Game/FirstPerson/Blueprints/BP_FirstPersonCharacter Object Reference"))
  (set `self.PlayerCharacter` PlayerCharacter)
  (set `self.Interacted Already` true))

(event `EventObjectInUse`
  (params (PlayerCharacter :type "/Game/FirstPerson/Blueprints/BP_FirstPersonCharacter Object Reference"))
  (if (`KismetSystemLibrary.IsValid` PlayerCharacter)
    (set `/Game/FirstPerson/Blueprints/BP_FirstPersonCharacter.ObjInUse` true (`self.PlayerCharacter`))))

(fn `GetInteractableType`
  (returns (`Actor Enum` :type "/Game/Alex/Blueprints/Enum_Interactive_Object_Types Enum"))
  ;[1 1 1] Allows us to classify which Monster to Spawn. False Line should spawn the Monster while true spawns nothing because this object has already been interacted with.
  (if (`self.Interacted Already`)
    (return "NewEnumerator3")
    (else
      (return "NewEnumerator3"))))

(fn `UserConstructionScript`)