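; BP_Interactable is an interactable object Blueprint that shows a widget prompt when something enters its sphere trigger.
; Begin overlap shows the widget if the object has not been interacted with; end overlap hides it only while the cutscene-playing flag is set.
; A RemoveOverlay event sets the Cube's overlay material to OriginalMaterial.
; The E-press cutscene playback and viewport widget creation are disconnected and never run.
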(event `self.ReceiveBeginPlay`)

(event `self.Sphere.OnComponentBeginOverlap`
  (params (OverlappedComponent :type "PrimitiveComponent Object Reference") (OtherActor :type "Actor Object Reference") (OtherComp :type "PrimitiveComponent Object Reference") (OtherBodyIndex :type Integer) (bFromSweep :type Boolean) (SweepResult :type "HitResult Structure (by ref)"))
  (if (not (`self.HasInteractedwith?`))
    (`SceneComponent.SetVisibility` (`self.Widget`) true false)
    (set `self.IsWidgetVisible?` true)))

(event `RemoveOverlay`
  (`MeshComponent.SetOverlayMaterial` (`self.Cube`) (`self.Original Material`)))

(event `self.Sphere.OnComponentEndOverlap`
  (params (OverlappedComponent :type "PrimitiveComponent Object Reference") (OtherActor :type "Actor Object Reference") (OtherComp :type "PrimitiveComponent Object Reference") (OtherBodyIndex :type Integer))
  (if (`self.CutSceneIsPLaying?`)
    (`SceneComponent.SetVisibility` (`self.Widget`) false false)
    (set `self.IsWidgetVisible?` false)))

(fn `UserConstructionScript`)